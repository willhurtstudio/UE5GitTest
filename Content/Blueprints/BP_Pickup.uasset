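; BP_Pickup is a collectible actor that awards an amount to the third-person character on touch.
; A Box overlap casts the other actor to BP_ThirdPersonCharacter, passes IncreaseAmount to its CollectPickup, then destroys the pickup.
; Any other overlapping actor only triggers a debug print of the overlapped component's name.
; The construction script prints the actor's location and applies the M_Door material to the Sphere.
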(event OnComponentBeginOverlap(Box)
  (params (OverlappedComponent :type Primitive%20Component%20Object%20Reference) (OtherActor :type Actor%20Object%20Reference) (OtherComp :type Primitive%20Component%20Object%20Reference) (OtherBodyIndex :type Integer) (bFromSweep :type Boolean) (SweepResult :type Hit%20Result%20Structure%20%28by%20ref%29))
  (bind _asbp_third_person_character (Utilities|Casting|CastToBP_ThirdPersonCharacter OtherActor)
    (:then
      (Default|CollectPickup _asbp_third_person_character (Variables|Default|GetIncrease%20Amount))
      (Actor|DestroyActor))
    (:CastFailed
      (Development|PrintString (Utilities|GetDisplayName OverlappedComponent)))))

(event EventBeginPlay)

(event Collision|EventActorBeginOverlap
  (params (OtherActor :type Actor%20Object%20Reference)))

(event EventTick
  (params (DeltaSeconds :type Float%20%28single-precision%29)))

(fn ConstructionScript
  (Development|PrintString (Utilities|String|ToString(Vector) (Transformation|GetActorLocation)))
  (Rendering|Material|SetMaterial (Variables|Default|GetSphere) 0 "/Game/StarterContent/Props/Materials/M_Door.M_Door"))